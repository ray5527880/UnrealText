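; Player-only free roam ability in the turn-based tile toolkit that moves the owning unit to a clicked tile.
; Activation and deactivation switch the turn state, with deactivation also reactivating the active unit.
; Clicks run pathfinding limited by the unit's max search range, then move it along the found path and start queued actions.
; AI assessment scores zero, and AI activation only prints a warning.
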(event EventClick
  (params (Index :type Integer) (Location :type Vector :default "0, 0, 0") (Key :type Key%20Structure) (bReleased :type Boolean) (ClickType :type EClickType%20Enum :default "NewEnumerator0"))
  (bind _owningunit (Variables|Default|GetOwningUnit))
  (bind (_bfoundatleastone _foundgridindexes _pathsmap) (Default|RunPathfindingUntilIndexFound (Variables|Default|GetGridManagerRef) (Variables|/Game/AdvancedTurnBasedTileToolkit/Core/Units/BP_Unit.BP_Unit_C|GetGridIndex _owningunit) (Variables|/Game/AdvancedTurnBasedTileToolkit/Core/Units/BP_Unit.BP_Unit_C|GetMaxSearchRange _owningunit) (Variables|/Game/AdvancedTurnBasedTileToolkit/Core/Units/BP_Unit.BP_Unit_C|GetPathfindingType _owningunit) (Utilities|Array|MakeArray Index)))
  (if _bfoundatleastone
    (Default|MovetoIndex (Variables|Default|GetOwningUnit) (Utilities|Array|Get(acopy) _foundgridindexes) _pathsmap)
    (if (Utilities|IsValid (Variables|Default|GetOwningUnit))
      (Default|InitializeQueuedActions (Variables|/Game/AdvancedTurnBasedTileToolkit/Core/BP_ATBTT_State.BP_ATBTT_State_C|GetActionManager (Variables|Default|GetGameStateRef))))))

(event EventDeactivateAbility
  (Variables|/Game/AdvancedTurnBasedTileToolkit/Core/BP_ATBTT_State.BP_ATBTT_State_C|SetTurnState (Variables|Default|GetGameStateRef) "NewEnumerator5")
  (Default|ReactivateActiveUnit (Variables|/Game/AdvancedTurnBasedTileToolkit/Core/BP_ATBTT_State.BP_ATBTT_State_C|GetTurnManager (Variables|Default|GetGameStateRef))))

(event EventPlayerActivate
  (params (Unit :type BP%20Unit%20Object%20Reference))
  (Variables|/Game/AdvancedTurnBasedTileToolkit/Core/BP_ATBTT_State.BP_ATBTT_State_C|SetTurnState (Variables|Default|GetGameStateRef) "NewEnumerator10"))

(event EventAIActivate
  (params (Unit :type BP%20Unit%20Object%20Reference))
  (Development|PrintString "WARNING: AI unit attempting to use player only FreeRoam skill" true true "(R=1.000000,G=1.000000,B=0.000000,A=1.000000)"))

(event EventAssessAbilityValue
  (params (Unit :type BP%20Unit%20Object%20Reference))
  (Default|CallOnAbilityAssesmentDone 0.0))

(fn ConstructionScript
  (|CallParentFunction))