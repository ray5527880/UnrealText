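; Experimental move ability for the turn-based tile toolkit, letting players click a reachable tile or drag a custom path from the unit.
; Activation runs pathfinding to mark reachable tiles and feed hover previews.
; Dragging uses a delayed loop to extend or trim the path within Move range, drawn as a spline.
; AI paths toward the closest faction-filtered unit, then picks the least dangerous nearby tile via BP_CoverSystem.
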(event Custom|Client_DisplayPath
  (params (PathLocations :type Array%20of%20Vectors))
  (bind _gridmanagerref (Variables|Default|GetGridManagerRef))
  (bind _pathspline (Variables|/Game/AdvancedTurnBasedTileToolkit/Core/Grid/BP_GridManager.BP_GridManager_C|GetPathSpline _gridmanagerref))
  ;[1 0 0] EXPERIMENTAL: This is blueprint is a work in progress, and mainly included as a starting point for developers.
  ;;[0 0 0] Animate Actions
  (Spline|SetSplinePoints _pathspline PathLocations "World" true)
  (Default|DisplayPathasSpline (Variables|Default|GetGridManagerRef) _pathspline PathLocations))

(event Custom|DragHover
  (bind _gridmanagerref (Variables|Default|GetGridManagerRef))
  (bind _dragpathcosts (Variables|Default|GetDragPathCosts))
  (bind _dragpathindexes (Variables|Default|GetDragPathIndexes))
  (bind _hoveredtile (Variables|Default|GetHoveredTile))
  (bind _hoveredtile_2 (Variables|Default|GetHoveredTile))
  (bind _returnvalue (Utilities|Array|FindItem _dragpathindexes _hoveredtile_2))
  (bind _gridunits (Variables|/Game/AdvancedTurnBasedTileToolkit/Core/Grid/BP_GridManager.BP_GridManager_C|GetGridUnits _gridmanagerref))
  (bind (_value _returnvalue_2) (Utilities|Map|Find _gridunits _hoveredtile))
  (bind _returnvalue_3 (+ _returnvalue 1))
  ;[1 0 0] EXPERIMENTAL: This is blueprint is a work in progress, and mainly included as a starting point for developers.
  ;;[0 0 0] Hover
  ;;;[0.5844 0.5149 0.2039] Drag Hover
  (CallFunction|ClientClearPath)
  (Utilities|Array|Clear (Variables|Default|GetDragPathIndexes))
  (Variables|Default|SetPathCost 0)
  (Variables|Default|SetDragIndex (Variables|/Game/AdvancedTurnBasedTileToolkit/Core/Units/BP_Unit.BP_Unit_C|GetGridIndex (Variables|Default|GetOwningUnit)))
  (Utilities|WhileLoopDelayed true 0.0
    (:Loop%20Body
      (Default|GetHitTileLocationandIndex (Variables|Default|GetGridManagerRef))
      (if (!= (Variables|Default|GetHoveredTile) (Variables|Default|GetDragIndex))
        (if (== (Variables|/Game/AdvancedTurnBasedTileToolkit/Core/Units/BP_Unit.BP_Unit_C|GetGridIndex (Variables|Default|GetOwningUnit)) (Variables|Default|GetHoveredTile))
          (CallFunction|StopDragHover false)
          (CallFunction|DragHover)
          (elif (not (Utilities|Array|ContainsItem (Variables|Default|GetDragPathIndexes) (Variables|Default|GetHoveredTile)))
            (if (.ReturnValue (Utilities|Map|Find (.edges (Utilities|Array|Get(acopy) (Variables|/Game/AdvancedTurnBasedTileToolkit/Core/Grid/BP_GridManager.BP_GridManager_C|GetGridEdges (Variables|Default|GetGridManagerRef)) (Variables|Default|GetDragIndex))) (Variables|Default|GetHoveredTile)))
              (if (<= (+ (Variables|Default|GetPathCost) (.Value (Utilities|Map|Find (.edges (Utilities|Array|Get(acopy) (Variables|/Game/AdvancedTurnBasedTileToolkit/Core/Grid/BP_GridManager.BP_GridManager_C|GetGridEdges (Variables|Default|GetGridManagerRef)) (Variables|Default|GetDragIndex))) (Variables|Default|GetHoveredTile)))) (Variables|/Game/AdvancedTurnBasedTileToolkit/Core/Units/BP_Unit.BP_Unit_C|GetMove (Variables|Default|GetOwningUnit)))
                (if _returnvalue_2
                  (if (Utilities|Set|Contains (Variables|/Game/AdvancedTurnBasedTileToolkit/Core/Units/BP_Unit.BP_Unit_C|GetAlliedFactions _value) (Variables|/Game/AdvancedTurnBasedTileToolkit/Core/Units/BP_Unit.BP_Unit_C|GetFaction (Variables|Default|GetOwningUnit)))
                    (if (Utilities|Enum|Equal(Enum) (Variables|/Game/AdvancedTurnBasedTileToolkit/Core/Units/BP_Unit.BP_Unit_C|GetPathfindingType (Variables|Default|GetOwningUnit)) "NewEnumerator1")
                      (bind _output_get (Variables|Default|SetPathCost (+ (Variables|Default|GetPathCost) (.Value (Utilities|Map|Find (.edges (Utilities|Array|Get(acopy) (Variables|/Game/AdvancedTurnBasedTileToolkit/Core/Grid/BP_GridManager.BP_GridManager_C|GetGridEdges (Variables|Default|GetGridManagerRef)) (Variables|Default|GetDragIndex))) (Variables|Default|GetHoveredTile)))) :!label _label))
                      (Utilities|Array|Add (Variables|Default|GetDragPathCosts) _output_get)
                      (Utilities|Array|Add (Variables|Default|GetDragPathIndexes) (Variables|Default|GetHoveredTile))
                      (Variables|Default|SetDragIndex (Variables|Default|GetHoveredTile) :!label _label_2)))
                  (else
                    (goto _label)))
                (Utilities|Array|Clear (Variables|Default|GetDragPathIndexesReversed))
                (bind _arrayelement (Utilities|Array|ReverseforEachLoop (Variables|Default|GetDragPathIndexes))
                  (:LoopBody
                    (Utilities|Array|Add (Variables|Default|GetDragPathIndexesReversed) _arrayelement)
                    (bind _pathlocations (Default|CreateSplinePath (Variables|Default|GetGridManagerRef) (Variables|Default|GetDragPathIndexesReversed) (Variables|/Game/AdvancedTurnBasedTileToolkit/Core/Units/BP_Unit.BP_Unit_C|GetBigUnitOffset (Variables|Default|GetOwningUnit))))
                    (CallFunction|ClientDisplayPath _pathlocations)))))
            (else
              (Utilities|Array|Resize (Variables|Default|GetDragPathCosts) _returnvalue_3)
              (Utilities|Array|Resize (Variables|Default|GetDragPathIndexes) _returnvalue_3)
              (Variables|Default|SetPathCost (Utilities|Array|Get(acopy) _dragpathcosts (Utilities|Array|LastIndex _dragpathcosts)))
              (goto _label_2))))))))

(event Custom|SpawnTileMarkers
  (params (OwningUnit :type BP%20Unit%20Object%20Reference) (Locations :type Array%20of%20Vectors))
  (bind _gridmanagerref (Variables|Default|GetGridManagerRef))
  ;[1 0 0] EXPERIMENTAL: This is blueprint is a work in progress, and mainly included as a starting point for developers.
  ;;[0 0 0] Animate Actions
  ;;;[0 0.2764 1] Spawn Tile Markers
  (Utilities|OwnsUnit OwningUnit
    (:true
      (Default|SpawnTileMarkersatLocations (Variables|Default|GetGridManagerRef) Locations (Variables|/Game/AdvancedTurnBasedTileToolkit/Core/Grid/BP_GridManager.BP_GridManager_C|GetbUseDecals _gridmanagerref) (Variables|/Game/AdvancedTurnBasedTileToolkit/Core/Grid/BP_GridManager.BP_GridManager_C|GetTileInMoveRangeDecalT _gridmanagerref) (Variables|/Game/AdvancedTurnBasedTileToolkit/Core/Grid/BP_GridManager.BP_GridManager_C|GetTileInMoveRangeMC _gridmanagerref)))))

(event Custom|StopDragHover
  (params (bClearPath :type Boolean))
  (bind _gridmanagerref (Variables|Default|GetGridManagerRef))
  (bind _dragpathcosts (Variables|Default|GetDragPathCosts))
  (bind _dragpathindexes (Variables|Default|GetDragPathIndexes))
  (bind _hoveredtile (Variables|Default|GetHoveredTile))
  (bind _hoveredtile_2 (Variables|Default|GetHoveredTile))
  (bind _returnvalue (Utilities|Array|FindItem _dragpathindexes _hoveredtile_2))
  (bind _gridunits (Variables|/Game/AdvancedTurnBasedTileToolkit/Core/Grid/BP_GridManager.BP_GridManager_C|GetGridUnits _gridmanagerref))
  (bind (_value _returnvalue_2) (Utilities|Map|Find _gridunits _hoveredtile))
  (bind _returnvalue_3 (+ _returnvalue 1))
  ;[1 0 0] EXPERIMENTAL: This is blueprint is a work in progress, and mainly included as a starting point for developers.
  ;;[0 0 0] Hover
  ;;;[0.5844 0.5149 0.2039] Drag Hover
  (if bClearPath
    (CallFunction|ClientClearPath))
  (Variables|Default|SetbIsDragging false)
  (Utilities|WhileLoopDelayed true 0.0) ; enters at Break
)

(event Custom|ClickEmptyTile
  (bind _owningunit (Variables|Default|GetOwningUnit))
  (bind _targetindex (Variables|Default|GetTargetIndex))
  (bind _storedpathsmap (Variables|Default|GetStoredPathsMap))
  (bind _value (Utilities|Map|Find _storedpathsmap _targetindex))
  ;[1 0 0] EXPERIMENTAL: This is blueprint is a work in progress, and mainly included as a starting point for developers.
  ;;[0 0 0] Click
  ;;;[0 0.04285 0.515] Click Empty Tile
  ;;;;[0 0 0] Prepare and Initialize Movement
  (if (and (>= (* (Variables|/Game/AdvancedTurnBasedTileToolkit/Core/Units/BP_Unit.BP_Unit_C|GetCurrentAP _owningunit) (Variables|/Game/AdvancedTurnBasedTileToolkit/Core/Units/BP_Unit.BP_Unit_C|GetMove _owningunit)) (.cost _value)) (> (.cost _value) 0))
    (Variables|/Game/AdvancedTurnBasedTileToolkit/Core/Units/BP_Unit.BP_Unit_C|SetCurrentAP (Variables|Default|GetOwningUnit) (Math|Integer|Max(Integer) (- (Variables|/Game/AdvancedTurnBasedTileToolkit/Core/Units/BP_Unit.BP_Unit_C|GetCurrentAP (Variables|Default|GetOwningUnit)) (+ (/ (- (.cost (.Value (Utilities|Map|Find (Variables|Default|GetStoredPathsMap) (Variables|Default|GetTargetIndex)))) 1) (Variables|/Game/AdvancedTurnBasedTileToolkit/Core/Units/BP_Unit.BP_Unit_C|GetMove (Variables|Default|GetOwningUnit))) 1))))
    (CallFunction|ExecuteAbility (Variables|Default|GetTargetIndex))))

(event EventAnimateAction
  (params (Action :type F%20Action%20Structure))
  (bind (_executingobject _actionname _binstantdeactivate _atcustomindex _bwithprevious _activationdelay _booleans _integers _floats _strings _vectors _transforms _actors _units) (Utilities|Struct|BreakFAction Action))
  ;[1 0 0] EXPERIMENTAL: This is blueprint is a work in progress, and mainly included as a starting point for developers.
  ;;[0 0 0] Animate Actions
  (switch name _actionname
    (:Default
      (|CallParentFunction Action))
    (:DisplayMoveTiles
      (CallFunction|SpawnTileMarkers (Utilities|Array|Get(acopy) _units) _vectors))))

(event EventFoundNoValidTarget
  ;[1 0 0] EXPERIMENTAL: This is blueprint is a work in progress, and mainly included as a starting point for developers.
  ;;[0 0 0] AI
  (Variables|/Game/AdvancedTurnBasedTileToolkit/Core/Units/BP_Unit.BP_Unit_C|SetCurrentAP (Variables|Default|GetOwningUnit) 0)
  (Default|ReactivateActiveUnit (Variables|/Game/AdvancedTurnBasedTileToolkit/Core/BP_ATBTT_State.BP_ATBTT_State_C|GetTurnManager (Variables|Default|GetGameStateRef))))

(event EventDeactivateAbility
  ;[1 0 0] EXPERIMENTAL: This is blueprint is a work in progress, and mainly included as a starting point for developers.
  ;;[0 0 0] Deactivate
  (|CallParentFunction)
  (Class|BPIBig|ToggleOffset(Message) (Game|GetPlayerController 0) false))

(event EventHover
  (params (Index :type Integer) (Location :type Vector :default "0, 0, 0"))
  ;[1 0 0] EXPERIMENTAL: This is blueprint is a work in progress, and mainly included as a starting point for developers.
  ;;[0 0 0] Hover
  (|CallParentFunction Index Location)
  (if (not (Variables|Default|GetbIsDragging))
    (CallFunction|ClientClearPath)
    (if (>= (Variables|Default|GetHoveredTile) 0)
      (if (not (Default|IsTileImpassable (Variables|Default|GetGridManagerRef) (Variables|Default|GetHoveredTile))) ; Never show path if tile is impassable
        (if (not (Utilities|Map|Contains (Variables|/Game/AdvancedTurnBasedTileToolkit/Core/Grid/BP_GridManager.BP_GridManager_C|GetGridUnits (Variables|Default|GetGridManagerRef)) (Variables|Default|GetHoveredTile)))
          (if (> (.cost (.Value (Utilities|Map|Find (Variables|Default|GetStoredPathsMap) (Variables|Default|GetHoveredTile)))) 0) ; Only show path if the current tile has a move cost (e.g. is reachable)
            (bind _pathlocations (Default|FindandDisplayPath (Variables|Default|GetGridManagerRef) (Variables|Default|GetStoredPathsMap) (Variables|Default|GetHoveredTile) false (Variables|/Game/AdvancedTurnBasedTileToolkit/Core/Grid/BP_GridManager.BP_GridManager_C|GetbDisplayPathAsSpline (Variables|Default|GetGridManagerRef)) (Variables|/Game/AdvancedTurnBasedTileToolkit/Core/Units/BP_Unit.BP_Unit_C|GetBigUnitOffset (Variables|Default|GetOwningUnit)))) ; Find and show a path from the path hovered to the tile the pathfinding array was generated from (generally the current pawn)
            (CallFunction|ClientDisplayPath _pathlocations)))))))

(event EventClick
  (params (Index :type Integer) (Location :type Vector :default "0, 0, 0") (Key :type Key%20Structure) (bReleased :type Boolean) (ClickType :type EClickType%20Enum :default "NewEnumerator0"))
  ;[1 0 0] EXPERIMENTAL: This is blueprint is a work in progress, and mainly included as a starting point for developers.
  ;;[0 0 0] Click
  (Variables|Default|SetTargetIndex Index)
  (switch Utilities|FlowControl|Switch|SwitchonEClickType ClickType
    (:NewEnumerator0
      (if bReleased
        (if (Variables|Default|GetbIsDragging)
          (CallFunction|ClientClearPath)
          (if (and (Utilities|Array|ContainsItem (Variables|Default|GetDragPathIndexes) (Variables|Default|GetTargetIndex)) (not (Utilities|Map|Contains (Variables|/Game/AdvancedTurnBasedTileToolkit/Core/Grid/BP_GridManager.BP_GridManager_C|GetGridUnits (Variables|Default|GetGridManagerRef)) (Variables|Default|GetTargetIndex))))
            (CallFunction|ExecuteAbility (Variables|Default|GetTargetIndex)))
          (CallFunction|StopDragHover true))
        (elif (== (Variables|Default|GetTargetIndex) (Variables|/Game/AdvancedTurnBasedTileToolkit/Core/Units/BP_Unit.BP_Unit_C|GetGridIndex (Variables|Default|GetOwningUnit)))
          (Variables|Default|SetbIsDragging true)
          (CallFunction|DragHover)
          (else
            (Variables|Default|SetbIsDragging false)
            (if (Utilities|Map|Contains (Variables|/Game/AdvancedTurnBasedTileToolkit/Core/Grid/BP_GridManager.BP_GridManager_C|GetGridUnits (Variables|Default|GetGridManagerRef)) (Variables|Default|GetTargetIndex))
              (CallFunction|DefaultClick (Variables|Default|GetTargetIndex) "0, 0, 0")
              (else
                (CallFunction|ClickEmptyTile)))))))
    (:NewEnumerator1
      (CallFunction|StopDragHover true))))

(event EventPlayerActivate
  (params (Unit :type BP%20Unit%20Object%20Reference))
  (bind _gridmanagerref (Variables|Default|GetGridManagerRef))
  (bind _owningunit (Variables|Default|GetOwningUnit))
  ;[1 0 0] EXPERIMENTAL: This is blueprint is a work in progress, and mainly included as a starting point for developers.
  ;;[0 0 0] Player Activate
  (if (> (Variables|/Game/AdvancedTurnBasedTileToolkit/Core/Units/BP_Unit.BP_Unit_C|GetCurrentAP Unit) 0)
    (Variables|Default|SetbDisplayInvalidTiles false)
    (|CallParentFunction (Variables|Default|GetOwningUnit))
    (bind _pathsmap (Default|RunPathfinding (Variables|Default|GetGridManagerRef) (Variables|/Game/AdvancedTurnBasedTileToolkit/Core/Units/BP_Unit.BP_Unit_C|GetGridIndex _owningunit) (Variables|Default|GetPossibleMove) (Variables|/Game/AdvancedTurnBasedTileToolkit/Core/Units/BP_Unit.BP_Unit_C|GetPathfindingType _owningunit)))
    (Variables|Default|SetStoredPathsMap _pathsmap)
    (Utilities|Array|Clear (Variables|Default|GetNearLocations))
    (bind _keys (Utilities|Map|Keys (Variables|Default|GetStoredPathsMap)))
    (if (> (Variables|/Game/AdvancedTurnBasedTileToolkit/Core/Units/BP_Unit.BP_Unit_C|GetSize (Variables|Default|GetOwningUnit)) 1)
      (bind _biggridindexes (Default|FindBigIndexesfromIndexes (Variables|Default|GetGridManagerRef) _keys (Variables|/Game/AdvancedTurnBasedTileToolkit/Core/Units/BP_Unit.BP_Unit_C|GetSize (Variables|Default|GetOwningUnit))))
      (Variables|Default|SetMoveDisplayIndexes _biggridindexes)
      (else
        (Variables|Default|SetMoveDisplayIndexes _keys)))
    (for _array_element (Variables|Default|GetMoveDisplayIndexes)
      (if (not (Utilities|Map|Contains (Variables|/Game/AdvancedTurnBasedTileToolkit/Core/Grid/BP_GridManager.BP_GridManager_C|GetGridUnits (Variables|Default|GetGridManagerRef)) _array_element))
        (Utilities|Array|Add (Variables|Default|GetNearLocations) (Math|Vector|MakeVector (.x (.Value (Utilities|Map|Find (Variables|/Game/AdvancedTurnBasedTileToolkit/Core/Grid/BP_GridManager.BP_GridManager_C|GetGridLocations _gridmanagerref) _array_element))) (.y (.Value (Utilities|Map|Find (Variables|/Game/AdvancedTurnBasedTileToolkit/Core/Grid/BP_GridManager.BP_GridManager_C|GetGridLocations _gridmanagerref) _array_element))) (+ (.z (.Value (Utilities|Map|Find (Variables|/Game/AdvancedTurnBasedTileToolkit/Core/Grid/BP_GridManager.BP_GridManager_C|GetGridLocations _gridmanagerref) _array_element))) (Variables|/Game/AdvancedTurnBasedTileToolkit/Core/Grid/BP_GridManager.BP_GridManager_C|GetTileInRangeZOffset _gridmanagerref))))))
    (Utilities|QueueAction false self "DisplayMoveTiles" true -1 false 0.0 0 0 0 0 (Variables|Default|GetNearLocations) 0 0 (Utilities|Array|MakeArray (Variables|Default|GetOwningUnit)))
    (else
      (Default|EndTurn (Variables|/Game/AdvancedTurnBasedTileToolkit/Core/BP_ATBTT_State.BP_ATBTT_State_C|GetTurnManager (Variables|Default|GetGameStateRef)) true true "NewEnumerator0" true true))))

(event EventAssessAbilityValue
  (params (Unit :type BP%20Unit%20Object%20Reference))
  ;[1 0 0] EXPERIMENTAL: This is blueprint is a work in progress, and mainly included as a starting point for developers.
  ;;[0 0 0] AI
  (Default|CallOnAbilityAssesmentDone 0.001))

(event EventExecuteAbility
  (params (TargetIndex :type Integer))
  ;[1 0 0] EXPERIMENTAL: This is blueprint is a work in progress, and mainly included as a starting point for developers.
  ;;[0 0 0] Click
  ;;;[0 0.04285 0.515] Click Empty Tile
  (|CallParentFunction TargetIndex)
  (CallFunction|PayAPCost false)
  (Utilities|QueueAction false (Variables|/Game/AdvancedTurnBasedTileToolkit/Core/BP_ATBTT_State.BP_ATBTT_State_C|GetTurnManager (Variables|Default|GetGameStateRef)) "SelectUnit" true -1 false 0.0 0 0 0 0 0 0 0 (Utilities|Array|MakeArray (Variables|Default|GetOwningUnit)))
  (if (Variables|Default|GetbIsDragging)
    (Default|MoveCustomPath (Variables|Default|GetOwningUnit) (Variables|Default|GetDragPathIndexesReversed))
    (else
      (Default|MovetoIndex (Variables|Default|GetOwningUnit) (Variables|Default|GetTargetIndex) (Variables|Default|GetStoredPathsMap))))
  (if (Utilities|IsValid (Variables|Default|GetOwningUnit))
    (Default|ReactivateActiveUnit (Variables|/Game/AdvancedTurnBasedTileToolkit/Core/BP_ATBTT_State.BP_ATBTT_State_C|GetTurnManager (Variables|Default|GetGameStateRef)))))

(event EventAIActivate
  (params (Unit :type BP%20Unit%20Object%20Reference))
  (bind _owningunit (Variables|Default|GetOwningUnit))
  (bind _owningunit_2 (Variables|Default|GetOwningUnit))
  ;[1 0 0] EXPERIMENTAL: This is blueprint is a work in progress, and mainly included as a starting point for developers.
  ;;[0 0 0] AI
  (bind _bmeetsrequirements (CallFunction|CheckRequirements))
  (if _bmeetsrequirements
    (bind (_btargetfound _closestunitindex _btargetbehindfriendlyunit _distancetoclosesttarget _pathsmap) (Default|FindClosestUnitinMoveRange (Variables|Default|GetGridManagerRef) (Variables|/Game/AdvancedTurnBasedTileToolkit/Core/Units/BP_Unit.BP_Unit_C|GetGridIndex _owningunit_2) (Variables|/Game/AdvancedTurnBasedTileToolkit/Core/Units/BP_Unit.BP_Unit_C|GetMaxSearchRange _owningunit_2) (Variables|/Game/AdvancedTurnBasedTileToolkit/Core/Units/BP_Unit.BP_Unit_C|GetPathfindingType _owningunit_2) (Variables|/Game/AdvancedTurnBasedTileToolkit/Core/Units/BP_Unit.BP_Unit_C|GetAlliedFactions _owningunit_2) true true))
    (if _btargetfound
      (bind _pathindexes (Default|FindPathtoIndex (Variables|Default|GetGridManagerRef) _pathsmap _closestunitindex))
      (bind (_bpathfound _closestindex) (Default|FindReachableIndexClosesttoTarget (Variables|Default|GetGridManagerRef) _pathindexes (Variables|/Game/AdvancedTurnBasedTileToolkit/Core/Units/BP_Unit.BP_Unit_C|GetPathfindingType (Variables|Default|GetOwningUnit)) (Variables|Default|GetPossibleMove) _distancetoclosesttarget _pathsmap))
      (if _bpathfound
        (Variables|Default|SetStoredPathsMap _pathsmap)
        (Utilities|Array|Clear (Variables|Default|GetAIMoveTargets))
        (Utilities|Array|Clear (Variables|Default|GetAIMoveTargetValues))
        (bind _pathsmap_2 (Default|RunPathfinding (Variables|Default|GetGridManagerRef) _closestindex (Variables|Default|GetPossibleMove) (Variables|/Game/AdvancedTurnBasedTileToolkit/Core/Units/BP_Unit.BP_Unit_C|GetPathfindingType (Variables|Default|GetOwningUnit))))
        (bind _keys (Utilities|Map|Keys _pathsmap_2))
        (for _array_element _keys
          (if (or (Math|Boolean|ANDBoolean (> (.cost (.Value (Utilities|Map|Find (Variables|Default|GetStoredPathsMap) _array_element))) 0) (<= (.cost (.Value (Utilities|Map|Find (Variables|Default|GetStoredPathsMap) _array_element))) (* (Variables|/Game/AdvancedTurnBasedTileToolkit/Core/Units/BP_Unit.BP_Unit_C|GetCurrentAP _owningunit) (Variables|/Game/AdvancedTurnBasedTileToolkit/Core/Units/BP_Unit.BP_Unit_C|GetMove _owningunit))) (not (Utilities|Map|Contains (Variables|/Game/AdvancedTurnBasedTileToolkit/Core/Grid/BP_GridManager.BP_GridManager_C|GetGridUnits (Variables|Default|GetGridManagerRef)) _array_element))) (== _array_element (Variables|/Game/AdvancedTurnBasedTileToolkit/Core/Units/BP_Unit.BP_Unit_C|GetGridIndex (Variables|Default|GetOwningUnit))))
            (Utilities|Array|Add (Variables|Default|GetAIMoveTargets) _array_element)
            (bind _value (Default|AssessTileDangerValue (Actor|GetComponentbyClass (Variables|Default|GetGridManagerRef) "/Game/AdvancedTurnBasedTileToolkit/Core/Grid/BP_CoverSystem.BP_CoverSystem_C") _array_element (Variables|/Game/AdvancedTurnBasedTileToolkit/Core/Units/BP_Unit.BP_Unit_C|GetFaction (Variables|Default|GetOwningUnit))))
            (Utilities|Array|Add (Variables|Default|GetAIMoveTargetValues) (- 1.0 _value))))
        (Variables|Default|SetTargetIndex (Utilities|Array|Get(acopy) (Variables|Default|GetAIMoveTargets) (.IndexOfMaxValue (Math|Float|MaxOfFloatArray (Variables|Default|GetAIMoveTargetValues)))))
        (if (!= (Variables|/Game/AdvancedTurnBasedTileToolkit/Core/Units/BP_Unit.BP_Unit_C|GetGridIndex (Variables|Default|GetOwningUnit)) (Variables|Default|GetTargetIndex))
          (Variables|/Game/AdvancedTurnBasedTileToolkit/Core/Units/BP_Unit.BP_Unit_C|SetCurrentAP (Variables|Default|GetOwningUnit) (Math|Integer|Max(Integer) (- (Variables|/Game/AdvancedTurnBasedTileToolkit/Core/Units/BP_Unit.BP_Unit_C|GetCurrentAP (Variables|Default|GetOwningUnit)) (+ (/ (- (.cost (.Value (Utilities|Map|Find (Variables|Default|GetStoredPathsMap) (Variables|Default|GetTargetIndex)))) 1) (Variables|/Game/AdvancedTurnBasedTileToolkit/Core/Units/BP_Unit.BP_Unit_C|GetMove (Variables|Default|GetOwningUnit))) 1))))
          (CallFunction|ExecuteAbility (Variables|Default|GetTargetIndex))
          (else
            (CallFunction|FoundNoValidTarget)))
        (else
          (CallFunction|FoundNoValidTarget)))
      (else
        (CallFunction|FoundNoValidTarget)))
    (else
      (CallFunction|FoundNoValidTarget))))

(fn ConstructionScript
  (|CallParentFunction))

(fn FindTargetValue
  (params (TargetIndex :type Integer))
  (return (/ 1.0 (Variables|/Game/AdvancedTurnBasedTileToolkit/Core/Units/BP_Unit.BP_Unit_C|GetCurrentHealth (.Value (Utilities|Map|Find (Variables|/Game/AdvancedTurnBasedTileToolkit/Core/Grid/BP_GridManager.BP_GridManager_C|GetGridUnits (Variables|Default|GetGridManagerRef)) TargetIndex))))))

(fn GetDescription
  (return "Move: 
Move to a tile within range."))