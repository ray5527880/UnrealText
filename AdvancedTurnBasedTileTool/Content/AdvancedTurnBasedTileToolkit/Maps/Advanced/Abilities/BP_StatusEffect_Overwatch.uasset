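; Overwatch status effect that gives its unit a one-time reaction shot at a non-allied unit entering a tile within range and line of sight.
; During simulation it resolves hit and damage through the owner's laser ability, multicasts the result, then disables; it also expires on turn start.
; During animation it matches the stored turn, path index and unit, then queues the shot with brief slow motion on the target, serialized by an "overwatch" delay lock.
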(event Custom|AnimateAttack
  (params (Unit :type BP%20Unit%20Object%20Reference) (PathIndex :type Integer))
  (bind _returnvalue (Game|GetGameState))
  (bind _asbp_atbtt_state (Utilities|Casting|CastToBP_ATBTT_State _returnvalue))
  (bind _turnmanager (Variables|/Game/AdvancedTurnBasedTileToolkit/Core/BP_ATBTT_State.BP_ATBTT_State_C|GetTurnManager _asbp_atbtt_state))
  (bind _delays (Variables|/Game/AdvancedTurnBasedTileToolkit/Core/BP_ATBTT_State.BP_ATBTT_State_C|GetDelays _asbp_atbtt_state))
  ;[1 0 0] Animate Attack
  (if (== PathIndex (Variables|Default|GetPathIndex))
    (if (== (Variables|Default|GetTurnOfActivation) (Variables|/Game/AdvancedTurnBasedTileToolkit/Core/BP_TurnManager.BP_TurnManager_C|GetCurrentTurnAnimate _turnmanager))
      (if (== (Variables|Default|GetTargetUnit) (Variables|/Game/AdvancedTurnBasedTileToolkit/Core/BP_TurnManager.BP_TurnManager_C|GetActiveUnitAnimate _turnmanager))
        (Variables|Default|SetTargetUnit Unit)
        (Utilities|DelayWhile (Utilities|Set|Contains _delays "overwatch")
          (:Continue
            (Utilities|Set|Add _delays "overwatch")
            (bind _array_element (Utilities|Array|ForEachLoopwithBreak (Variables|/Game/AdvancedTurnBasedTileToolkit/Core/Units/BP_AbilitySystem.BP_AbilitySystem_C|GetAbilityRefs (Actor|GetComponentbyClass (Variables|Default|GetOwningUnit) "/Game/AdvancedTurnBasedTileToolkit/Core/Units/BP_AbilitySystem.BP_AbilitySystem_C")) :!label _label)
              (:LoopBody
                (bind _asbp_ability_laser (Utilities|Casting|CastToBP_Ability_Laser _array_element))
                (Utilities|FlowControl|Sequence
                  (:then_0
                    (goto _label Break))
                  (:then_1
                    (EventDispatchers|UnbindEventfromOnUnitEnterTileAnimate (Variables|Default|GetGridManagerRef) (delegate Custom|AnimateAttack))
                    (Utilities|QueueAction true _asbp_ability_laser "Shoot" false -1 false 0.0 (Utilities|Array|MakeArray (Variables|Default|GetbHitStored)) 0 (Utilities|Array|MakeArray (Variables|Default|GetDamageStored)) 0 0 0 0 (Utilities|Array|MakeArray (Variables|Default|GetOwningUnit) (Variables|Default|GetTargetUnit)))
                    (Variables|/Game/AdvancedTurnBasedTileToolkit/Core/Units/BP_Unit.BP_Unit_C|SetSpeedModifier (Variables|Default|GetTargetUnit) 0.1)
                    (Variables|/Script/Engine.Actor|SetCustomTimeDilation (Variables|Default|GetTargetUnit) 0.1)
                    (Utilities|FlowControl|Delay 2.0)
                    (Variables|/Game/AdvancedTurnBasedTileToolkit/Core/Units/BP_Unit.BP_Unit_C|SetSpeedModifier (Variables|Default|GetTargetUnit) 1.0)
                    (Variables|/Script/Engine.Actor|SetCustomTimeDilation (Variables|Default|GetTargetUnit) 1.0)
                    (Class|BPICameraControls|FollowActor(Message) (Game|Player|GetPlayerPawn 0) (Variables|Default|GetTargetUnit))
                    (Utilities|Set|Remove (Variables|/Game/AdvancedTurnBasedTileToolkit/Core/BP_ATBTT_State.BP_ATBTT_State_C|GetDelays (.AsBP%20ATBTT%20State (Utilities|Casting|CastToBP_ATBTT_State (Game|GetGameState)))) "overwatch")
                    (Rendering|SetActorHiddenInGame true)))))))))))

(event Custom|Multicast_BindOnUnitEnter
  (params (PathIndex :type Integer) (TurnOfActivation :type Integer) (TargetUnit :type BP%20Unit%20Object%20Reference) (Hit_Stored :type Boolean) (DamageStored :type Float%20%28single-precision%29))
  ;[1 0 0] Animate Attack
  (EventDispatchers|BindEventtoOnUnitEnterTileAnimate (Variables|Default|GetGridManagerRef) (delegate Custom|AnimateAttack))
  (Variables|Default|SetPathIndex PathIndex)
  (Variables|Default|SetTurnOfActivation TurnOfActivation)
  (Variables|Default|SetTargetUnit TargetUnit)
  (Variables|Default|SetbHitStored Hit_Stored)
  (Variables|Default|SetDamageStored DamageStored))

(event Custom|CheckOverwatch
  (params (Unit :type BP%20Unit%20Object%20Reference) (GridIndex :type Integer) (PathIndex :type Integer))
  (bind _owningunit (Variables|Default|GetOwningUnit))
  (bind _gridmanagerref (Variables|Default|GetGridManagerRef))
  ;[1 0.5778 0] Check Overwatch - Simulate
  (Variables|Default|SetTargetUnit Unit)
  (Variables|Default|SetPathIndex PathIndex)
  (if (not (Utilities|Set|Contains (Variables|/Game/AdvancedTurnBasedTileToolkit/Core/Units/BP_Unit.BP_Unit_C|GetAlliedFactions (Variables|Default|GetOwningUnit)) (Variables|/Game/AdvancedTurnBasedTileToolkit/Core/Units/BP_Unit.BP_Unit_C|GetFaction Unit)))
    (if (< (Default|FindDistanceIinTilesBetweenIndexes _gridmanagerref (Variables|/Game/AdvancedTurnBasedTileToolkit/Core/Units/BP_Unit.BP_Unit_C|GetGridIndex _owningunit) (Variables|/Game/AdvancedTurnBasedTileToolkit/Core/Units/BP_Unit.BP_Unit_C|GetGridIndex (Variables|Default|GetTargetUnit)) false) (Variables|Default|GetRange))
      (bind _bvisible (Default|CheckifTileIsVisiblefromOtherTile (Variables|Default|GetGridManagerRef) (Variables|/Game/AdvancedTurnBasedTileToolkit/Core/Units/BP_Unit.BP_Unit_C|GetGridIndex _owningunit) (Variables|/Game/AdvancedTurnBasedTileToolkit/Core/Units/BP_Unit.BP_Unit_C|GetGridIndex (Variables|Default|GetTargetUnit)) (* (Default|FindDistanceIinTilesBetweenIndexes _gridmanagerref (Variables|/Game/AdvancedTurnBasedTileToolkit/Core/Units/BP_Unit.BP_Unit_C|GetGridIndex _owningunit) (Variables|/Game/AdvancedTurnBasedTileToolkit/Core/Units/BP_Unit.BP_Unit_C|GetGridIndex (Variables|Default|GetTargetUnit)) false) (Variables|/Game/AdvancedTurnBasedTileToolkit/Core/Grid/BP_GridManager.BP_GridManager_C|GetTileXSize _gridmanagerref)) (Default|FindDistanceIinTilesBetweenIndexes _gridmanagerref (Variables|/Game/AdvancedTurnBasedTileToolkit/Core/Units/BP_Unit.BP_Unit_C|GetGridIndex _owningunit) (Variables|/Game/AdvancedTurnBasedTileToolkit/Core/Units/BP_Unit.BP_Unit_C|GetGridIndex (Variables|Default|GetTargetUnit)) false) 0 true))
      (if _bvisible
        (if (> (Variables|/Game/AdvancedTurnBasedTileToolkit/Core/Units/BP_Unit.BP_Unit_C|GetCurrentHealth (Variables|Default|GetTargetUnit)) 0.0)
          (bind _turnmanager (Class|BPISingletons|GetTurnManager(Message) (Game|GetGameState)))
          (Variables|Default|SetTurnOfActivation (Variables|/Game/AdvancedTurnBasedTileToolkit/Core/BP_TurnManager.BP_TurnManager_C|GetCurrentTurn _turnmanager))
          (bind _array_element (Utilities|Array|ForEachLoopwithBreak (Variables|/Game/AdvancedTurnBasedTileToolkit/Core/Units/BP_AbilitySystem.BP_AbilitySystem_C|GetAbilityRefs (Actor|GetComponentbyClass (Variables|Default|GetOwningUnit) "/Game/AdvancedTurnBasedTileToolkit/Core/Units/BP_AbilitySystem.BP_AbilitySystem_C")) :!label _label)
            (:LoopBody
              (bind _asbp_ability_laser (Utilities|Casting|CastToBP_Ability_Laser _array_element))
              (Utilities|FlowControl|Sequence
                (:then_0
                  (goto _label Break))
                (:then_1
                  (EventDispatchers|UnbindEventfromOnUnitEnterTileSimulate (Variables|Default|GetGridManagerRef) (delegate Custom|CheckOverwatch))
                  (bind (_bhit _targetunit _damage) (Default|ShootUnit _asbp_ability_laser (Variables|Default|GetOwningUnit) (Variables|Default|GetTargetUnit) false))
                  (Variables|Default|SetbHitStored _bhit)
                  (Variables|Default|SetDamageStored _damage)
                  (CallFunction|MulticastBindonUnitEnter (Variables|Default|GetPathIndex) (Variables|Default|GetTurnOfActivation) (Variables|Default|GetTargetUnit) (Variables|Default|GetbHitStored) (Variables|Default|GetDamageStored))
                  (CallFunction|Disable))))))))))

(event EventDisable
  (|CallParentFunction)
  (EventDispatchers|UnbindEventfromOnUnitEnterTileSimulate (Variables|Default|GetGridManagerRef) (delegate Custom|CheckOverwatch)))

(event EventRunonTurnStart
  (|CallParentFunction)
  (CallFunction|Disable))

(event EventActivate
  (params (Target%20Unit :type BP%20Unit%20Object%20Reference))
  ;[1 0.5778 0] Check Overwatch - Simulate
  (|CallParentFunction Target%20Unit)
  (EventDispatchers|BindEventtoOnUnitEnterTileSimulate (Variables|Default|GetGridManagerRef) (delegate Custom|CheckOverwatch)))

(fn ConstructionScript
  (|CallParentFunction))