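; Animated Medic unit Blueprint for the Advanced maps of the Advanced Turn Based Tile Toolkit.
; Its construction script runs the parent's, then switches on Faction to set the helmet, legs and torso materials and the unit icon, using red material variants for Enemy.
; The event graph holds only disabled stub events, so the file adds no runtime logic of its own.
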(event EventBeginPlay
  (|CallParentFunction))

(event Collision|EventActorBeginOverlap
  (params (OtherActor :type Actor%20Object%20Reference))
  (|CallParentFunction OtherActor))

(event EventTick
  (params (DeltaSeconds :type Float%20%28single-precision%29))
  (|CallParentFunction DeltaSeconds))

(fn ConstructionScript
  (|CallParentFunction)
  (switch Utilities|FlowControl|Switch|SwitchonEFaction (Variables|Default|GetFaction)
    (:NewEnumerator0
      (Rendering|Material|SetMaterial (Variables|Character|GetMesh) 0 "/Game/AdvancedTurnBasedTileToolkit/Maps/Advanced/Units/M_Medic_Helmet.M_Medic_Helmet")
      (Rendering|Material|SetMaterial (Variables|Character|GetMesh) 1 "/Game/AdvancedTurnBasedTileToolkit/Maps/Advanced/Units/M_Medic_Legs.M_Medic_Legs")
      (Rendering|Material|SetMaterial (Variables|Character|GetMesh) 2 "/Game/AdvancedTurnBasedTileToolkit/Maps/Advanced/Units/M_Medic_Torso.M_Medic_Torso")
      (Variables|Default|SetIcon "/Game/AdvancedTurnBasedTileToolkit/Maps/Advanced/Units/T_UnitIcon_Medic_01.T_UnitIcon_Medic_01"))
    (:NewEnumerator1
      (Rendering|Material|SetMaterial (Variables|Character|GetMesh) 0 "/Game/AdvancedTurnBasedTileToolkit/Maps/Advanced/Units/M_Medic_Helmet_Red.M_Medic_Helmet_Red")
      (Rendering|Material|SetMaterial (Variables|Character|GetMesh) 1 "/Game/AdvancedTurnBasedTileToolkit/Maps/Advanced/Units/M_Medic_Legs_Red.M_Medic_Legs_Red")
      (Rendering|Material|SetMaterial (Variables|Character|GetMesh) 2 "/Game/AdvancedTurnBasedTileToolkit/Maps/Advanced/Units/M_Medic_Torso_Red.M_Medic_Torso_Red")
      (Variables|Default|SetIcon "/Game/AdvancedTurnBasedTileToolkit/Maps/Advanced/Units/T_UnitIcon_Medic_02.T_UnitIcon_Medic_02"))))