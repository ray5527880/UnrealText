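; Hydra attack ability for the 2D turn-based tile toolkit that strikes a target tile once per head of the owning unit.
; Activation caches the head count from the Hydra unit.
; Execution pays AP, then for each head rechecks the tile for a unit, queues a melee action and applies damage immediately without auto-animation.
; Finally, the turn manager reactivates the active unit.
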(event EventExecuteAbility
  (params (TargetIndex :type Integer))
  (bind _owningunit (Variables|Default|GetOwningUnit))
  (bind _asbp_unit_2d (Utilities|Casting|CastToBP_Unit_2D _owningunit))
  (Variables|Default|SetMoveTargetIndex TargetIndex)
  (CallFunction|PayAPCost false)
  (Utilities|FlowControl|ForLoopwithBreak 1 (Variables|Default|GetNumHeads)
    (:LoopBody
      (Utilities|IsValid (.Value (Utilities|Map|Find (Variables|/Game/AdvancedTurnBasedTileToolkit/Core/Grid/BP_GridManager.BP_GridManager_C|GetGridUnits (Variables|Default|GetGridManagerRef)) (Variables|Default|GetMoveTargetIndex)))
        (:Is%20Valid
          (Utilities|QueueAction false self "Melee" false -1 false 0.0 0 0 (Utilities|Array|MakeArray (Variables|Default|GetDamage)) 0 0 0 0 (Utilities|Array|MakeArray (Variables|Default|GetOwningUnit) (.Value (Utilities|Map|Find (Variables|/Game/AdvancedTurnBasedTileToolkit/Core/Grid/BP_GridManager.BP_GridManager_C|GetGridUnits (Variables|Default|GetGridManagerRef)) (Variables|Default|GetMoveTargetIndex)))) (Utilities|Array|MakeArray (Variables|/Game/AdvancedTurnBasedTileToolkit/Maps/2D/Units/BP_Unit_2D.BP_Unit_2D_C|GetProjectile _asbp_unit_2d) (Variables|/Game/AdvancedTurnBasedTileToolkit/Maps/2D/Units/BP_Unit_2D.BP_Unit_2D_C|GetAttackSound _asbp_unit_2d) (Variables|/Game/AdvancedTurnBasedTileToolkit/Maps/2D/Units/BP_Unit_2D.BP_Unit_2D_C|GetHitSound _asbp_unit_2d)))
          (Default|TakeDamage (.Value (Utilities|Map|Find (Variables|/Game/AdvancedTurnBasedTileToolkit/Core/Grid/BP_GridManager.BP_GridManager_C|GetGridUnits (Variables|Default|GetGridManagerRef)) (Variables|Default|GetMoveTargetIndex))) (Variables|Default|GetDamage) false))))
    (:Completed
      (Default|ReactivateActiveUnit (Variables|/Game/AdvancedTurnBasedTileToolkit/Core/BP_ATBTT_State.BP_ATBTT_State_C|GetTurnManager (Variables|Default|GetGameStateRef))))))

(event EventActivate
  (params (OwningUnit :type BP%20Unit%20Object%20Reference) (bReassess :type Boolean))
  (bind _asbp_unit_2d_hydra (Utilities|Casting|CastToBP_Unit_2D_Hydra OwningUnit)
    (:then
      (Variables|Default|SetNumHeads (Variables|/Game/AdvancedTurnBasedTileToolkit/Maps/2D/Units/BP_Unit_2D_Hydra.BP_Unit_2D_Hydra_C|GetHeads _asbp_unit_2d_hydra)))
    (:CastFailed
      _))
  (|CallParentFunction OwningUnit bReassess))

(fn ConstructionScript
  (|CallParentFunction))