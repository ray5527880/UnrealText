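; A 2D bridge grid actor that raises once enough torches are lit, making its tile passable.
; Each AttemptRaise call increments a lit-torch counter and compares it to the required count.
; On reaching it, the grid manager opens the tile at cost 1 and a Raise action is queued, whose animation step unhides the paper sprite.
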(event Custom|AttemptRaise
  (Math|Integer|IncrementInt (Variables|Default|GetCurrentTorchesLit)
    (:%20%20
      (if (>= (Variables|Default|GetCurrentTorchesLit) (Variables|Default|GetRequiredTorchesLit))
        (Default|MakeTilePassable (Variables|Default|GetGridManagerRef) (Variables|Default|GetGridIndex) 1)
        (Utilities|QueueAction false self "Raise" true -1 false 0.0)))))

(event EventAnimateAction
  (params (Action :type F%20Action%20Structure))
  (Development|SetHiddeninGame (Variables|Default|GetPaperSprite) false false))

(fn ConstructionScript
  (|CallParentFunction))