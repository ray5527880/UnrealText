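; Child grid manager for the toolkit's 2D map that adds fog of war and triggers grid objects when units end movement.
; Activation covers each tile with an instanced plane.
; RevealTiles uses range queries and wall line traces to find visible tiles, wakes stealthed units there, and queues an action that drops their fog planes.
; Movement-range edges border only revealed tiles, while a custom pathfinding step stops expanding at occupied tiles.
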(event Custom|EndOnObjects
  (params (Unit :type BP%20Unit%20Object%20Reference) (GridIndex :type Integer))
  (CallFunction|InteractwithObjects GridIndex Unit 0 true "NewEnumerator0" -1))

(event EventAnimateAction
  (params (Action :type F%20Action%20Structure))
  (bind (_executingobject _actionname _binstantdeactivate _atcustomindex _bwithprevious _activationdelay _booleans _integers) (Utilities|Struct|BreakFAction Action))
  (switch name _actionname
    (:Default
      (|CallParentFunction Action))
    (:RevealTiles
      (for _array_element _integers
        (Components|InstancedStaticMesh|UpdateInstanceTransform (Variables|Default|GetFogOfWar) _array_element (Math|Transform|MakeTransform "0, 0,-100.000000" "0, 0, 0" "1,1,1") false true false)))))

(event EventActivateGridManager
  (|CallParentFunction)
  (EventDispatchers|BindEventtoOnUnitEndMovementSimulate (delegate Custom|EndOnObjects))
  (bind _returnvalue (AddComponent|AddInstancedStaticMeshComponent false))
  (bind _output_get (Variables|Default|SetFogOfWar _returnvalue))
  (Components|StaticMesh|SetStaticMesh _output_get "/Game/AdvancedTurnBasedTileToolkit/Core/Grid/SM_SimplePlane.SM_SimplePlane")
  (bind _turnmanager (Class|BPISingletons|GetTurnManager(Message) (Game|GetGameState)))
  (Variables|/Game/AdvancedTurnBasedTileToolkit/Core/BP_TurnManager.BP_TurnManager_C|SetUnitActivationDelay _turnmanager 0.1)
  (for _index (range 0 (- (Variables|Default|GetGridSizeSquared) 1))
    (Components|InstancedStaticMesh|AddInstance (Variables|Default|GetFogOfWar) (Math|Transform|MakeTransform (Math|Vector|MakeVector (.x (CallFunction|ConvertIndextoLocationSquareGrid _index)) (.y (CallFunction|ConvertIndextoLocationSquareGrid _index)) (+ (.z (CallFunction|ConvertIndextoLocationSquareGrid _index)) 2e+01)) "0, 0, 0" "1,1,1"))))

(fn ConstructionScript
  (|CallParentFunction))

(fn RevealTiles
  (params (GridIndex :type Integer))
  (bind _gridindexes (CallFunction|FindVisibleTilesandWallsinRange GridIndex))
  (for _array_element _gridindexes
    (if (.ReturnValue (Utilities|Map|Find (Variables|Default|GetGridUnits) _array_element))
      (Default|Wake (Actor|GetComponentbyClass (.Value (Utilities|Map|Find (Variables|Default|GetGridUnits) _array_element)) "/Game/AdvancedTurnBasedTileToolkit/Core/Units/BP_UnitStealthComponent.BP_UnitStealthComponent_C")))
    (if (not (Utilities|Set|Contains (Variables|Default|GetRevealedGridIndexes) _array_element))
      (Utilities|Set|Add (Variables|Default|GetRevealedGridIndexes) _array_element)
      (for _array_element_2 (Class|InstancedStaticMeshComponent|GetInstancesOverlappingSphere (Variables|Default|GetFogOfWar) (CallFunction|ConvertfromGridtoWorld (CallFunction|ConvertIndextoLocationSquareGrid _array_element)) 2e+01 true)
        (Utilities|Array|Add (LocalVariables|GetInstanceIndexes) _array_element_2))))
  (Utilities|QueueAction false self "RevealTiles" true -1 false 0.0 0 (LocalVariables|GetInstanceIndexes))
  (return))

(fn FindVisibleTilesandWallsinRange
  (params (StartIndex :type Integer))
  (bind _gridlocations (Variables|Default|GetGridLocations))
  (bind _value (Utilities|Map|Find _gridlocations StartIndex))
  (bind (_x _y _z) (Math|Vector|BreakVector _value))
  (bind _inrangetiles (CallFunction|GetIndexesinRange StartIndex 6 false false))
  (for _array_element _inrangetiles
    (bind (_outhit _returnvalue) (Collision|LineTraceByChannel (CallFunction|ConvertfromGridtoWorld (Math|Vector|MakeVector _x _y (+ _z (Variables|Default|GetTraceForWallsHeight)))) (CallFunction|ConvertfromGridtoWorld (Math|Vector|MakeVector (.X (Math|Vector|BreakVector (CallFunction|ConvertIndextoLocationSquareGrid (.index _array_element)))) (.Y (Math|Vector|BreakVector (CallFunction|ConvertIndextoLocationSquareGrid (.index _array_element)))) (+ (.Z (Math|Vector|BreakVector (CallFunction|ConvertIndextoLocationSquareGrid (.index _array_element)))) (Variables|Default|GetTraceForWallsHeight)))) "TraceTypeQuery4" false 0 "None" false)) ; Do not add tiles that are blocked from sight from collision volumes blocking RangeTrace.
    (if _returnvalue
      (if (Math|Vector|Equal(Vector) (.location _outhit) (CallFunction|ConvertIndextoLocationSquareGrid (.index _array_element)) (* (Variables|Default|GetTileXSize) 1.42))
        (Utilities|Array|Add (LocalVariables|GetFoundIndexes) (.index _array_element) :!label _label))
      (else
        (goto _label))))
  (return (LocalVariables|GetFoundIndexes)))

(fn MakeEdgeMeshTransforms
  (params (EdgeIndexes :type Array%20of%20Integers) (PathsMap :type Map%20of%20Integers%20to%20Structs))
  (for _array_element EdgeIndexes
    (bind _integers (CallFunction|GetAdjacentIndexes _array_element false false))
    (for _array_element_2 _integers
      (if (not (Utilities|Map|Contains PathsMap _array_element_2))
        (if (Utilities|Set|Contains (Variables|Default|GetRevealedGridIndexes) _array_element_2)
          (Utilities|Array|Add (LocalVariables|GetLocalEdgeTransforms) (Math|Transform|MakeTransform (Math|Vector|MakeVector (.X (Math|Vector|BreakVector (.Value (Utilities|Map|Find (Variables|Default|GetGridLocations) _array_element)))) (.Y (Math|Vector|BreakVector (.Value (Utilities|Map|Find (Variables|Default|GetGridLocations) _array_element)))) (+ (.Z (Math|Vector|BreakVector (.Value (Utilities|Map|Find (Variables|Default|GetGridLocations) _array_element)))) (Variables|Default|GetTileInRangeZOffset))) (Math|Rotator|FindLookatRotation (CallFunction|ConvertIndextoLocationSquareGrid _array_element_2) (.Value (Utilities|Map|Find (Variables|Default|GetGridLocations) _array_element))) "1,1,1"))))))
  (return (LocalVariables|GetLocalEdgeTransforms)))

(fn SpawnEdgeMeshatTransform
  (params (Mesh :type Foliage%20Instanced%20Static%20Mesh%20Component%20Object%20Reference) (EdgeTransform :type Transform))
  (Components|InstancedStaticMesh|AddInstance Mesh EdgeTransform))

(fn SearchandAddAdjacentTilesCustom1
  (params (SearchStep :type Integer) (PathsMap :type Map%20of%20Integers%20to%20Structs) (ReachableUnits :type Set%20of%20Integers) (Move :type Integer) (OpenListTiles :type Array%20of%20F%20Pathfinding%20Structures) (DelayedSearchTiles :type Array%20of%20F%20Pathfinding%20Structures) (ContinuePathTiles :type Array%20of%20F%20Pathfinding%20Structures))
  (for _array_element OpenListTiles
    (if (== SearchStep (.cost _array_element)) ; If the parent tile cost is higher than the current search range, do not check now, but re-check next iteration
      (bind _keys (Utilities|Map|Keys (.edges (Utilities|Array|Get(acopy) (Variables|Default|GetGridEdges) (.index _array_element)))))
      (for _array_element_2 _keys
        (if (not (Utilities|Set|Contains (Variables|Default|GetSearchedTiles) _array_element_2)) ; Has the node already been searched (if so the cost should be > 0)
          (Utilities|Set|Add (Variables|Default|GetSearchedTiles) _array_element_2)
          (if (<= (+ (.Value (Utilities|Map|Find (.edges (Utilities|Array|Get(acopy) (Variables|Default|GetGridEdges) (.index _array_element))) _array_element_2)) (.cost _array_element)) Move)
            (Utilities|Map|Add PathsMap _array_element_2 (Utilities|Struct|MakeFPathfindingNew (+ (.Value (Utilities|Map|Find (.edges (Utilities|Array|Get(acopy) (Variables|Default|GetGridEdges) (.index _array_element))) _array_element_2)) (.cost _array_element)) (.index _array_element)))
            (if (Utilities|Map|Contains (Variables|Default|GetGridUnits) _array_element_2) ; Prevents units from walking through the spaces of other units\n(a variant that allows for movement through friendly units is\nshown in the Search and add adjacent tiles\n(Pass Through Friendlies) function).
              (Utilities|Set|Add ReachableUnits _array_element_2)
              (else
                (Utilities|Array|Add (LocalVariables|GetLocalOpenListChildTiles) (Utilities|Struct|MakeFPathfinding _array_element_2 (+ (.Value (Utilities|Map|Find (.edges (Utilities|Array|Get(acopy) (Variables|Default|GetGridEdges) (.index _array_element))) _array_element_2)) (.cost _array_element)) (.index _array_element)))))
            (else
              (Utilities|Array|Add ContinuePathTiles (Utilities|Struct|MakeFPathfinding _array_element_2 (+ (.Value (Utilities|Map|Find (.edges (Utilities|Array|Get(acopy) (Variables|Default|GetGridEdges) (.index _array_element))) _array_element_2)) (.cost _array_element)) (.index _array_element)))))))
      (else
        (Utilities|Array|Add DelayedSearchTiles (Utilities|Struct|MakeFPathfinding (.index _array_element) (.cost _array_element) (.parent _array_element))) ; If the movement cost is too high for this search step, save it for later search steps.
      )))
  (return (LocalVariables|GetLocalOpenListChildTiles)))