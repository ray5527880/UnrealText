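; BP_GridCamera_2D is the grid camera Blueprint for the 2D maps of the turn-based tile toolkit.
; Its Pan and Rotate events are empty, so neither performs any action here.
; A disconnected "Simple 2d Pan" node would offset the spring arm's relative X/Y location by axis input scaled by delta time, but it never runs.
; The construction script only calls the parent's.
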(event EventRotate
  (params (AxisValue :type Float%20%28single-precision%29)))

(event EventPan
  (params (AxisValue :type Vector%202D%20Structure))
  ;[1 0.5451 0] Simple 2d Pan
)

(fn ConstructionScript
  (|CallParentFunction))