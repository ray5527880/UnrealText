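; Equippable item for the 2D turn-based tile game that a hero unit picks up by interacting with it.
; On its first interaction with a hero, it passes its combat stats, sprite, equip type, sounds and projectile to the hero's Equip.
; It then queues its own Destroy action and a DestroyActors action on the game state's action manager.
; When animating its queued action, it hides itself and plays a potion sound.
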(event EventAnimateAction
  (params (Action :type F%20Action%20Structure))
  (switch name (.ActionName (Utilities|Struct|BreakFAction Action))
    (:Destroy
      (Rendering|SetActorHiddenInGame true)
      (Audio|PlaySound2D "/Game/AdvancedTurnBasedTileToolkit/Maps/2D/Items/A_Potion.A_Potion"))))

(event EventInteract
  (params (TriggeringActor :type Actor%20Object%20Reference) (InteractionType :type EInteract%20Enum :default "NewEnumerator0") (CurrentPathIndex :type Integer))
  (bind _asbp_unit_2d_hero (Utilities|Casting|CastToBP_Unit_2D_Hero TriggeringActor))
  (Utilities|FlowControl|DoOnce false
    (:Completed
      (Default|Equip _asbp_unit_2d_hero (Variables|Default|GetDamage) (Variables|Default|GetArmor) (Variables|Default|GetEquipSprite) (Variables|Default|GetEquipType) (Variables|Default|GetRange) (Variables|Default|GetAttackSound) (Variables|Default|GetHitSound) (Variables|Default|GetProjectile))
      (Utilities|QueueAction false self "Destroy" true -1 false 0.0)
      (bind _actionmanader (Class|BPISingletons|GetActionManager(Message) (Game|GetGameState)))
      (Utilities|QueueAction false _actionmanader "DestroyActors" true -1 false 0.0 0 0 0 0 0 0 (Utilities|Array|MakeArray self)))))

(fn ConstructionScript
  (|CallParentFunction))