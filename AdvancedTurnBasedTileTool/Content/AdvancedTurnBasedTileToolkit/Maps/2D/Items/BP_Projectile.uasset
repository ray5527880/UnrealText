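; BP_Projectile is a 2D projectile actor in the turn-based tile toolkit that flies a sprite to a target location.
; On BeginPlay it faces the target, applies its sprite and moves its root there, timing the move by distance over movement speed.
; On arrival it plays the hit sound, hides itself rather than being destroyed, and tells the game state that the action has ended.
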(event EventBeginPlay
  (bind _returnvalue (Transformation|GetActorLocation))
  (bind _target (Variables|Default|GetTarget))
  (Transformation|SetActorRotation (Math|Rotator|FindLookatRotation (Transformation|GetActorLocation) (Variables|Default|GetTarget)))
  (Rendering|Components|Sprite|SetSprite (Variables|Default|GetProjectileSprite) (Variables|Default|GetSprite))
  (Rendering|SetActorHiddenInGame false)
  (Components|MoveComponentTo (Variables|Default|GetDefaultSceneRoot) _target (Math|Rotator|FindLookatRotation _returnvalue _target) false false (/ (Math|Vector|VectorLength (- _target _returnvalue)) (Variables|Default|GetMovementSpeed)) false)
  (Audio|PlaySound2D (Variables|Default|GetHitSound))
  (Rendering|SetActorHiddenInGame true)
  (Class|BPIAction|EndAction(Message) (Game|GetGameState)))

(fn ConstructionScript)