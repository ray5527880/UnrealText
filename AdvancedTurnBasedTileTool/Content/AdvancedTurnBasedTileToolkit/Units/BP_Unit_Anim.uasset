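; BP_Unit_Anim is an animated unit for the Advanced Turn Based Tile Toolkit that extends its parent unit with Animation Blueprint playback.
; On BeginPlay it caches the mesh's anim instance as ABP_Unit.
; Each movement timeline update calls a multicast event that passes CurrentSpeed to the anim Blueprint's AnimateMovement.
; AnimateUnit forwards the requested action to AnimateAbility.
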(event Custom|MulticastMoveAnimation
  (Default|AnimateMovement (Variables|Default|GetAbpRef) (Variables|Default|GetCurrentSpeed)))

(event EventAnimateUnit
  (params (Action :type F%20Action%20Structure%20%28by%20ref%29))
  (Default|AnimateAbility (Variables|Default|GetAbpRef) Action))

(event EventTimelineMoveUpdateFunc
  (|CallParentFunction)
  (CallFunction|MulticastMoveAnimation))

(event EventBeginPlay
  (|CallParentFunction)
  (bind _asabp_unit (Utilities|Casting|CastToABP_Unit (Components|SkeletalMesh|GetAnimInstance (Variables|Character|GetMesh))))
  (Variables|Default|SetAbpRef _asabp_unit))

(fn ConstructionScript
  (|CallParentFunction))